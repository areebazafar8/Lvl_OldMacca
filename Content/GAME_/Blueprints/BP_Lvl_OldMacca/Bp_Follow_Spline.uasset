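; Spline follower Blueprint for the OldMacca level that moves its REF component along a spline at a set Speed.
; Tick accumulates distance from Speed and delta time, then applies the spline's local location and rotation at that distance to REF, preserving its scale.
; With IsLooping on, distance snaps back to zero past the spline's end; otherwise it keeps accumulating.
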(event `self.ReceiveTick`
  (params (DeltaSeconds :type "Float (single-precision)"))
  (bind (_returnvalue_location _returnvalue_rotation) (`KismetMathLibrary.BreakTransform` (`SplineComponent.GetTransformAtDistanceAlongSpline` (`self.Spline`) (`self.Distance`) "Local" false)))
  (set `self.Distance` (+ (* DeltaSeconds (`self.Speed`)) (`self.Distance`)))
  (`SceneComponent.K2_SetRelativeTransform` (`self.REF`) (`KismetMathLibrary.MakeTransform` _returnvalue_location _returnvalue_rotation (`SceneComponent.RelativeScale3D` (`self.REF`))) false false)
  (if (`self.isLooping`)
    (if (> (`self.Distance`) (`SplineComponent.GetSplineLength` (`self.Spline`)))
      (set `self.Distance` 0.0))))

(fn `UserConstructionScript`)